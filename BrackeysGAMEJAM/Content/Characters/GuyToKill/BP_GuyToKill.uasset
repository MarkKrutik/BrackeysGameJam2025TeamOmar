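; BP_GuyToKill is a character that patrols a looping route through a list of points.
; On BeginPlay, MoveToTarget sends it by AI MoveTo to the current point's location.
; On success it waits for WaitTime, advances the index, wrapping to zero after the last point, and calls MoveToTarget again.
; A failed move has no handler, so the patrol stops there.
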(event `self.ReceiveBeginPlay`
  (`self.MoveToTarget`))

(event `MoveToTarget`
  ; Move To Target
  (`|AIMoveTo` self (.location (`|GetArrayItem` (`self.Points`) (`self.currentIndex`))) null
    (:`OnSuccess`
      (`KismetSystemLibrary.Delay` (`self.Wait Time`))
      (if (>= (`self.currentIndex`) (- (`KismetArrayLibrary.Array_Length` (`self.Points`)) 1))
        ;; Reset Index
        (set `self.currentIndex` 0)
        (else
          ;; Increment Index
          (set `self.currentIndex` (+ (`self.currentIndex`) 1))))
      (`self.MoveToTarget`))))

(fn `UserConstructionScript`)