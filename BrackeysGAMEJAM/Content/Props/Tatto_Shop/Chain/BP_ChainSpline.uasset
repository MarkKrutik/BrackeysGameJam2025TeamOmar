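; BP_ChainSpline is a spline placement prop, named for chains, that repeats a chosen mesh along a spline.
; The construction script sets PlaceMesh on an instanced static mesh and derives spacing from its bounding-box X size plus OffSet.
; It adds local-space instances at each spacing interval along the spline length, using GetLocationAtSpline for positions.
; Instances keep zero rotation, so they do not follow the spline's direction.
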(fn `Get Location at spline`
  (params (A :type "Float (double-precision)"))
  (returns (ReturnValue :type "Vector Structure"))
  (return (`SplineComponent.GetLocationAtDistanceAlongSpline` (`self.Spline`) (* A (`self.Spacing`)) "Local")))

(fn `UserConstructionScript`
  (bind (_min _max) (break `Box` (`StaticMesh.GetBoundingBox` (`self.PlaceMesh`))))
  (`StaticMeshComponent.SetStaticMesh` (`self.InstancedStaticMesh`) (`self.PlaceMesh`))
  (bind _output_get (set `self.Spacing` (+ (.x (- _max _min)) (`self.OffSet`))))
  (bind _output_get_2 (set `self.Number of Items` (`KismetMathLibrary.FFloor` (/ (`SplineComponent.GetSplineLength` (`self.Spline`)) _output_get))))
  (for _index (range (+ _output_get_2 1))
    (`InstancedStaticMeshComponent.AddInstance` (`self.InstancedStaticMesh`) (`KismetMathLibrary.MakeTransform` (`self.Get Location at spline` (`KismetMathLibrary.Conv_IntToDouble` _index))) false)))